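; BP_FlamePillar is a flame pillar actor that gives its fire light a changing, flickering intensity.
; From BeginPlay, ChooseTimeLine randomly picks one of two FlameIntensity timelines to play from the start.
; Each timeline update feeds ScaleFlameIntensity, which multiplies the curve value by BaseIntensity and sets it on FireLight.
; When a timeline finishes it calls ChooseTimeLine again, so the variation loops endlessly in random order.
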(event `self.ReceiveBeginPlay`
  (`self.ChooseTimeLine`))

(event `ChooseTimeLine`
  (switch `int` (`KismetMathLibrary.RandomIntegerInRange` 0 1)
    (:`Default`
      (`self.StartTimeline_2` :!label _label))
    (:`0`
      (`self.StartTimeline_1`))
    (:`1`
      (goto _label))))

(event `StartTimeline_1`
  (bind (_direction _flameintensity) (`Timeline|FlameIntensity_1` :!via `PlayFromStart`)
    (:`Update`
      (`self.ScaleFlameIntensity` _flameintensity))
    (:`Finished`
      (`self.ChooseTimeLine`))))

(event `StartTimeline_2`
  (bind (_direction _flameintensity) (`Timeline|FlameIntensity_2` :!via `PlayFromStart`)
    (:`Update`
      (`self.ScaleFlameIntensity` _flameintensity))
    (:`Finished`
      (`self.ChooseTimeLine`))))

(fn `ScaleFlameIntensity`
  (params (Intensity :type "Float (double-precision)"))
  (`LightComponent.SetIntensity` (`self.FireLight`) (* Intensity (`self.BaseIntensity`))))

(fn `UserConstructionScript`)