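; Base enemy character Blueprint that supplies spawn, attack-facing and dissolve presentation hooks.
; On BeginPlay, a timeline drives the uniform relative scale of the mesh as a spawn effect.
; UpdateFacingTarget feeds a location into Motion Warping as the "FacingTarget" warp target.
; Two events run separate body and weapon timelines that animate the "Dissolve" parameter on the dynamic material passed in.
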(event `self.ReceiveBeginPlay`
  (bind (_direction _scaletrack) (`Timeline|SpawnTimeLine`)
    (:`Update`
      (`SceneComponent.SetRelativeScale3D` (`self.Mesh`) (`KismetMathLibrary.MakeVector` _scaletrack _scaletrack _scaletrack)))))

(event `CombatInterface.UpdateFacingTarget`
  (params (Target :type "Vector Structure (by ref)"))
  (`MotionWarpingComponent.AddOrUpdateWarpTargetFromLocation` (`self.MotionWarping`) "FacingTarget" Target))

(event `self.StartDisolveTimeLine`
  (params (DynamicMaterialInstance :type "MaterialInstanceDynamic Object Reference"))
  (bind (_direction _dissolvetrack) (`Timeline|时间轴`)
    (:`Update`
      (`MaterialInstanceDynamic.SetScalarParameterValue` DynamicMaterialInstance "Dissolve" _dissolvetrack))))

(event `self.StartWeaponDisolveTimeLine`
  (params (DynamicMaterialInstance :type "MaterialInstanceDynamic Object Reference"))
  (bind (_direction _weapondissolvetrack) (`Timeline|时间轴_0`)
    (:`Update`
      (`MaterialInstanceDynamic.SetScalarParameterValue` DynamicMaterialInstance "Dissolve" _weapondissolvetrack))))

(fn `UserConstructionScript`)