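; GA_RangedAttack is an enemy gameplay ability that performs a montage-driven projectile attack on the avatar's combat target.
; It updates the motion-warp facing target through CombatInterface, then plays a random tagged attack montage.
; The montage's gameplay event spawns a projectile from the tagged socket toward the target's current location, with optional pitch override.
; The ability ends shortly after firing, or when the montage completes or is interrupted or cancelled.
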(event `self.K2_ActivateAbility`
  (bind _returnvalue (`self.GetAvatarActorFromActorInfo`))
  (bind _returnvalue_2 (message `EnemyInterface.GetCombatTarget` _returnvalue))
  (bind _ascombat_interface (cast `CombatInterface` _returnvalue)
    (:`then`
      (bind _returnvalue_3 (`Actor.K2_GetActorLocation` _returnvalue_2))
      (set `self.CombatTargetLocation` _returnvalue_3)
      ;[1 1 1] 设置 warp target
      (`CombatInterface.UpdateFacingTarget` _ascombat_interface _returnvalue_3)
      (bind _returnvalue_4 (message `CombatInterface.GetAttackMontages` (`self.GetAvatarActorFromActorInfo`)))
      (bind _output_get (set `self.TaggedMontage` (`self.GetRandomMontageFromArray` _returnvalue_4)))
      (bind (_montage _montagetag _combatsockettag) (break `TaggedMontage` _output_get))
      (`AbilityTask_PlayMontageAndWait.CreatePlayMontageAndWaitProxy` "None" _montage 1.0 "None" false
        (:`then`
          (`AbilityTask_WaitGameplayEvent.WaitGameplayEvent` _montagetag null true
            (:`EventReceived`
              (bind _returnvalue_5 (message `CombatInterface.GetCombatSocketLocation` (`self.GetAvatarActorFromActorInfo`) _combatsockettag))
              (bind _returnvalue_6 (message `EnemyInterface.GetCombatTarget` (`self.GetAvatarActorFromActorInfo`)))
              (`self.SpawnProjectile` (`Actor.K2_GetActorLocation` _returnvalue_6) _combatsockettag (`self.ShowOverridePitch`) (`self.PitchOverride`))
              (`KismetSystemLibrary.Delay` 0.5)
              (`self.K2_EndAbility`))))
        (:`OnCompleted`
          (`self.K2_EndAbility` :!label _label))
        (:`OnInterrupted`
          (goto _label))
        (:`OnCancelled`
          (goto _label))))
    (:`CastFailed`
      (`self.K2_EndAbility`))))